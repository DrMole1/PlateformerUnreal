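; BP_CameraShake is a camera shake Blueprint with a custom event, Saoul, that takes a Touch value but is empty.
; Disconnected nodes would rebuild the location and rotation oscillators as sine waves, adding Touch to the current pitch, yaw and roll amplitudes.
; That logic never runs, and a similar addition for vertical location amplitude is left unused, so the graph changes nothing.
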(event `Saoul`
  (params (Touch :type "Float (double-precision)")))